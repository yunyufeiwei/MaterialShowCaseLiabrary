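; Toon-rendering actor that shows a configurable static mesh with an outline, built entirely in the construction script.
; DuplicateMesh applies the mesh and optional material, then adds a second mesh component at the same transform, using OutlineMesh if valid or the main mesh otherwise.
; That duplicate gets a dynamic MI_Outline instance at MaterialIndex, driven by color, thickness, intensity and a shrink-over-distance toggle.
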(event EventBeginPlay)

(event Collision|EventActorBeginOverlap
  (params (OtherActor :type Actor%20Object%20Reference)))

(event EventTick
  (params (DeltaSeconds :type Float%20%28single-precision%29)))

(fn ConstructionScript
  (CallFunction|DuplicateMesh))

(fn DuplicateMesh
  (Components|StaticMesh|SetStaticMesh (Variables|Default|GetStaticMesh) (Variables|Mesh|GetYourMesh))
  (Utilities|IsValid (Variables|Mesh|GetMaterial)
    (:Is%20Valid
      (Rendering|Material|SetMaterial (Variables|Default|GetStaticMesh) (Variables|Default|GetMaterial%20Index) (Variables|Mesh|GetMaterial)))
    (:Is%20Not%20Valid
      _))
  (Utilities|IsValid (Variables|Mesh|GetOutlineMesh)
    (:Is%20Valid
      ;[1 1 1] 如果Outline有模型使用这里的逻辑
      (bind _returnvalue (AddComponent|AddStaticMeshComponent true (Transformation|GetWorldTransform (Variables|Default|GetStaticMesh))))
      (bind _output_get (Variables|Default|SetStatic%20Mesh%20Component _returnvalue))
      (Components|StaticMesh|SetStaticMesh _output_get (Variables|Mesh|GetOutlineMesh))
      (bind _returnvalue_2 (Rendering|Material|CreateDynamicMaterialInstance _output_get (Variables|Default|GetMaterial%20Index) "/Game/卡通渲染/MaterialInstance/MI_Outline.MI_Outline" "None" :!class /Script/Engine.PrimitiveComponent))
      (Utilities|FlowControl|Sequence
        (:then_0
          (Rendering|Material|SetVectorParameterValue _returnvalue_2 "Outline Color" (Variables|Outline|GetOutline%20Color) :!class /Script/Engine.MaterialInstanceDynamic)
          (Rendering|Material|SetScalarParameterValue _returnvalue_2 "Outline Thickness" (Variables|Outline|GetOutline%20Thickness) :!class /Script/Engine.MaterialInstanceDynamic)
          (Rendering|Material|SetScalarParameterValue _returnvalue_2 "OutLine Intensity" (Variables|Outline|GetOutLine%20Intensity) :!class /Script/Engine.MaterialInstanceDynamic))
        (:then_1
          (if (Variables|Outline|GetOutline%20Shrink%20Over%20Distance)
            (Rendering|Material|SetScalarParameterValue _returnvalue_2 "Outline Scale Over Distance" 1.0 :!class /Script/Engine.MaterialInstanceDynamic)
            (else
              (Rendering|Material|SetScalarParameterValue _returnvalue_2 "Outline Scale Over Distance" 0.0 :!class /Script/Engine.MaterialInstanceDynamic))))))
    (:Is%20Not%20Valid
      ;[1 1 1] 如果outline没有模型就使用这里的逻辑
      (bind _returnvalue_3 (AddComponent|AddStaticMeshComponent true (Transformation|GetWorldTransform (Variables|Default|GetStaticMesh))))
      (bind _output_get_2 (Variables|Default|SetStatic%20Mesh%20Component _returnvalue_3))
      (Components|StaticMesh|SetStaticMesh _output_get_2 (Variables|Mesh|GetYourMesh))
      (bind _returnvalue_4 (Rendering|Material|CreateDynamicMaterialInstance _output_get_2 (Variables|Default|GetMaterial%20Index) "/Game/卡通渲染/MaterialInstance/MI_Outline.MI_Outline" "None" :!class /Script/Engine.PrimitiveComponent))
      (Utilities|FlowControl|Sequence
        (:then_0
          (Rendering|Material|SetVectorParameterValue _returnvalue_4 "Outline Color" (Variables|Outline|GetOutline%20Color) :!class /Script/Engine.MaterialInstanceDynamic)
          (Rendering|Material|SetScalarParameterValue _returnvalue_4 "Outline Thickness" (Variables|Outline|GetOutline%20Thickness) :!class /Script/Engine.MaterialInstanceDynamic)
          (Rendering|Material|SetScalarParameterValue _returnvalue_4 "OutLine Intensity" (Variables|Outline|GetOutLine%20Intensity) :!class /Script/Engine.MaterialInstanceDynamic))
        (:then_1
          (if (Variables|Outline|GetOutline%20Shrink%20Over%20Distance)
            (Rendering|Material|SetScalarParameterValue _returnvalue_4 "Outline Scale Over Distance" 1.0 :!class /Script/Engine.MaterialInstanceDynamic)
            (else
              (Rendering|Material|SetScalarParameterValue _returnvalue_4 "Outline Scale Over Distance" 0.0 :!class /Script/Engine.MaterialInstanceDynamic))))))))
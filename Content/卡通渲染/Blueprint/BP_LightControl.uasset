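; Light controller actor for cel shading that drives a referenced directional light and a sky light from its own intensity and color variables.
; UpdateLight applies these values and mirrors them, plus the sun's forward vector, into MPC_CelShaderLightContronl, since materials cannot read the light's direction.
; The construction script aligns the directional light to the Arrow and calls UpdateLight if that light is valid.
; UpdateRealTime toggles Tick, which repeats UpdateLight without re-aligning.
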(event Custom|UpdateLight
  (bind _directionallight (Variables|DirectionalLight|GetDirectionalLight))
  (bind _skylightcomponent (Variables|SkyLight|GetSkyLightComponent))
  (bind _lightcomponent (Variables|/Script/Engine.Light|GetLightComponent _directionallight))
  (bind _lightcomponent_2 (Variables|/Script/Engine.Light|GetLightComponent _skylightcomponent))
  (bind _returnvalue (Transformation|GetWorldRotation _lightcomponent))
  (bind _returnvalue_2 (Math|Vector|GetForwardVector _returnvalue))
  (Utilities|FlowControl|Sequence
    (:then_0
      (Utilities|IsValid _directionallight
        (:Is%20Valid
          (Rendering|Components|Light|SetIntensity _lightcomponent (Variables|DirectionalLight|GetDirectionalLightIntensity))
          (Rendering|Components|Light|SetLightColor _lightcomponent (Variables|DirectionalLight|GetDirectionalLightColor) true)
          (Rendering|Material|SetVectorParameterValue "/Game/卡通渲染/Blueprint/MPC_CelShaderLightContronl.MPC_CelShaderLightContronl" "Directional Light Vector" (Utilities|Struct|MakeLinearColor (.x _returnvalue_2) (.y _returnvalue_2) (.z _returnvalue_2) 1.0) :!class /Script/Engine.KismetMaterialLibrary) ; 设置方向光的轴向，由于材质里面无法取到光源轴向，\n因此需要借用MPC，将xyz方向在材质与蓝图中传递
          (Rendering|Material|SetVectorParameterValue "/Game/卡通渲染/Blueprint/MPC_CelShaderLightContronl.MPC_CelShaderLightContronl" "Directional Light Color" (Variables|DirectionalLight|GetDirectionalLightColor) :!class /Script/Engine.KismetMaterialLibrary) ; 卡通渲染的着色模型，颜色受方向光影响，\n因此也使用MPC进行参数传递
          (Rendering|Material|SetScalarParameterValue "/Game/卡通渲染/Blueprint/MPC_CelShaderLightContronl.MPC_CelShaderLightContronl" "Directional Light Intensity" (Variables|DirectionalLight|GetDirectionalLightIntensity) :!class /Script/Engine.KismetMaterialLibrary) ; 卡通渲染的着色模型，方向光强度会有影响，\n因此也使用MPC进行参数传递
        )))
    (:then_1
      (Utilities|IsValid _skylightcomponent
        (:Is%20Valid
          (Rendering|Components|Light|SetIntensity _lightcomponent_2 (Variables|SkyLight|GetSkyLight%20Intensity))
          (Rendering|Components|Light|SetLightColor _lightcomponent_2 (Variables|SkyLight|GetSkyLight%20Color) true)
          (Rendering|Material|SetScalarParameterValue "/Game/卡通渲染/Blueprint/MPC_CelShaderLightContronl.MPC_CelShaderLightContronl" "SkyLightIntensity" (Variables|SkyLight|GetSkyLight%20Intensity) :!class /Script/Engine.KismetMaterialLibrary)
          (Rendering|Material|SetVectorParameterValue "/Game/卡通渲染/Blueprint/MPC_CelShaderLightContronl.MPC_CelShaderLightContronl" "SkyLight Color" (Variables|SkyLight|GetSkyLight%20Color) :!class /Script/Engine.KismetMaterialLibrary))))))

(event EventTick
  (params (DeltaSeconds :type Float%20%28single-precision%29))
  (CallFunction|UpdateLight))

(fn ConstructionScript
  (bind _directionallight (Variables|DirectionalLight|GetDirectionalLight))
  (bind _arrow (Variables|Default|GetArrow))
  (bind _returnvalue (Transformation|GetWorldRotation _arrow))
  (Actor|Tick|SetActorTickEnabled (Variables|Default|GetUpdateRealTime))
  (Utilities|IsValid _directionallight
    (:Is%20Valid
      (Transformation|SetActorRotation _directionallight (Math|Rotator|MakeRotator (.roll _returnvalue) (.pitch _returnvalue) (.yaw _returnvalue)))
      (CallFunction|UpdateLight))))